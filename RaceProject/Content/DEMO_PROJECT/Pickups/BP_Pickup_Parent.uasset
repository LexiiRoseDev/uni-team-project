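; Parent pickup Blueprint for the demo project that responds to actor overlaps and respawns after a short delay.
; If the overlapping actor's display name matches the demo sports car, it reports ItemID to BP_PC_DEMOPROJ and plays a 2D sound.
; Any overlapping actor hides the cube and triggers collect sound and confetti, except when that controller cast fails.
; CanPickup blocks repeat triggers until a timer shows the cube again.
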(event `self.ReceiveActorBeginOverlap`
  (params (OtherActor :type "Actor Object Reference"))
  (bind _returnvalue (`SceneComponent.K2_GetComponentLocation` (`self.Cube`)))
  (if (`self.CanPickup`)
    (if (== (`KismetSystemLibrary.GetDisplayName` OtherActor) "BP_P_SportsCar_DEMO0")
      (bind _asbp_pc_demoproj (cast `/Game/DEMO_PROJECT/BP_PC_DEMOPROJ` (`GameplayStatics.GetPlayerController` 0)))
      (`/Game/DEMO_PROJECT/BP_PC_DEMOPROJ.PickupCollected` _asbp_pc_demoproj (`self.ItemID`))
      (`GameplayStatics.PlaySound2D` "/Game/DEMO_PROJECT/SFX/SC_GoodTroy.SC_GoodTroy" 1.0 1.0 0.0 null null))
    (`SceneComponent.SetHiddenInGame` (`self.Cube`) true false)
    (set `self.CanPickup` false)
    (`KismetSystemLibrary.K2_SetTimerDelegate` (delegate `ShowPickup`) 5.0)
    (`GameplayStatics.PlaySoundAtLocation` "/Game/DEMO_PROJECT/SFX/SC_CollectNoise_Cue.SC_CollectNoise_Cue" _returnvalue (struct) 1.0 1.0 0.0 null null null null)
    (`NiagaraFunctionLibrary.SpawnSystemAtLocation` "/Game/DEMO_PROJECT/VFX/NS_ConfettiBurst.NS_ConfettiBurst" _returnvalue)))

(event `ShowPickup`
  (`SceneComponent.SetHiddenInGame` (`self.Cube`) false false)
  (set `self.CanPickup` true))

(fn `UserConstructionScript`)