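; BP_KartRender is the kart actor for the main menu's customisation screen, holding a side panel whose material can be swapped.
; On BeginPlay it registers itself with GM_MainMenu.
; CreateMaterial hands the kart to the game mode's CustomisationMenu and builds a dynamic instance of the base side material.
; ApplyMaterial assigns that instance to the side panel mesh.
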(event `self.ReceiveBeginPlay`
  (bind _asgm_main_menu (cast `/Game/MAIN_PROJECT/GM_MainMenu` (`GameplayStatics.GetGameMode`)))
  (set `/Game/MAIN_PROJECT/GM_MainMenu.KartRender` self _asgm_main_menu))

(event `CreateMaterial`
  (bind _asgm_main_menu (cast `/Game/MAIN_PROJECT/GM_MainMenu` (`GameplayStatics.GetGameMode`)))
  (set `/Game/MAIN_PROJECT/CustomisationMenu/WBP_CustomisationMenu.KartRender` self (`/Game/MAIN_PROJECT/GM_MainMenu.CustomisationMenu` _asgm_main_menu))
  (bind _returnvalue (`KismetMaterialLibrary.CreateDynamicMaterialInstance` (`self.BaseSideMat`) "SideMat"))
  (set `self.SideMaterial` _returnvalue))

(fn `ApplyMaterial`
  (`PrimitiveComponent.SetMaterial` (`self.SM_SidePanel`) 0 (`self.SideMaterial`)))

(fn `UserConstructionScript`)